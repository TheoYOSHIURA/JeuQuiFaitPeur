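; Tutorial VFX actor that keeps a multiple-tentacle effect component, NSTentacles31, wandering around the actor.
; On BeginPlay a timeline lerps the component's relative location from the origin to a point above it.
; Each time the timeline finishes, it picks a random target scaled by Range and stretched along Y, then replays from the last target for endless motion.
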(event EventBeginPlay
  (Variables|Default|SetNewPos "0.000000,0.000000,100.000000")
  (Variables|Default|SetOldPos "0, 0, 0")
  (bind _newtrack_0 (Timeline|Timeline PlayFromStart)
    (:Update
      (Transformation|SetRelativeLocation (Variables|Default|GetNS_Tentacles_31) (Math|Vector|Lerp(Vector) (Variables|Default|GetOldPos) (Variables|Default|GetNewPos) _newtrack_0) false false))
    (:Finished
      (Variables|Default|SetOldPos (Variables|Default|GetNewPos))
      (Variables|Default|SetNewPos (* (* (Math|Vector|ClampVectorSize (Math|Random|RandomUnitVector) 0.9 1.0) "1.000000,3.000000,1.000000") -1.0 (Variables|Default|GetRange)))
      (Timeline|Timeline PlayFromStart))))

(event EventTick
  (params (DeltaSeconds :type Float%20%28single-precision%29)))

(fn ConstructionScript)