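; Tutorial actor that spawns and restarts three Niagara tentacle effects.
; On BeginPlay, a helper function hides each placed Niagara component in game and spawns an auto-destroying copy of its system attached to it.
; Reset destroys the three spawned copies and spawns them again.
; The Off event is empty, and some single-tentacle spawn and destroy logic is left unconnected.
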(event Custom|Off)

(event Custom|Reset
  (Components|DestroyComponent (stale _newparam))
  (Components|DestroyComponent (stale _newparam_2))
  (Components|DestroyComponent (stale _newparam_3))
  (bind _newparam (CallFunction|NewFunction (Variables|Default|GetNS%20Tentacle%201)))
  (bind _newparam_2 (CallFunction|NewFunction (Variables|Default|GetNS%20Tentacle%202)))
  (bind _newparam_3 (CallFunction|NewFunction (Variables|Default|GetNS%20Tentacle%203))))

(event EventBeginPlay
  (bind _newparam (CallFunction|NewFunction (Variables|Default|GetNS%20Tentacle%201)))
  (bind _newparam_2 (CallFunction|NewFunction (Variables|Default|GetNS%20Tentacle%202)))
  (bind _newparam_3 (CallFunction|NewFunction (Variables|Default|GetNS%20Tentacle%203))))

(fn ConstructionScript)

(fn NewFunction
  (params (NS :type Niagara%20Component%20Object%20Reference))
  (Development|SetHiddeninGame NS true false)
  (bind _returnvalue (Niagara|SpawnSystemAttached (AssetData|GetAsset NS) NS "None" "0, 0, 0" "0, 0, 0" "KeepRelativeOffset" true))
  (return _returnvalue))