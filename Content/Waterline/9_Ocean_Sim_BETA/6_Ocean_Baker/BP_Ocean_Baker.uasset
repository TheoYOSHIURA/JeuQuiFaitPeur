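; Ocean baker actor that renders the Waterline ocean simulation into a flipbook grid in RT_Ocean_Bake.
; CaptureOcean re-runs on a looping timer, drawing scene captures cell by cell while stepping spectrum time across the capture length.
; Wave amplitude crossfades linearly from FFT controller 1 to controller 2 during the bake.
; The construction script fits capture and debug plane to the ocean tile and sets preview parameters and material.
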(event Custom|Capture%20Ocean
  (bind _flip_res (Variables|Default|GetFlip%20Res))
  (Utilities|FlowControl|Sequence
    (:then_0
      (Utilities|FlowControl|DoOnce false :!label _label
        (:Completed
          (Variables|Default|SetFlip%20Cells%20Current 0.0)
          (Variables|Default|SetCurrent%20Row 0.0)
          (Variables|Default|SetCurrent%20Column 0.0)
          (Variables|Default|SetNumber%20of%20Cells%20Rendered 0.0)
          (bind _output_get (Variables|Default|SetCapture%20Ocean%20Time 0.0))
          (Rendering|Material|SetScalarParameterValue "/Game/Waterline/9_Ocean_Sim_BETA/1_BP_Actors/1_Compute_Shaders/1_Spectrum_P_Collection.1_Spectrum_P_Collection" "Time Override" _output_get :!class /Script/Engine.KismetMaterialLibrary)
          (Rendering|Material|SetScalarParameterValue "/Game/Waterline/9_Ocean_Sim_BETA/1_BP_Actors/1_Compute_Shaders/1_Spectrum_P_Collection.1_Spectrum_P_Collection" "Time Bake" (Variables|Default|GetCapture%20Length%20%28s%29) :!class /Script/Engine.KismetMaterialLibrary)
          (Variables|Default|SetAmplitude%201 (Variables|Default|GetOcean%20Amplitude))
          (Variables|Default|SetAmplitude%202 0.0)
          (bind _returnvalue (Actor|GetActorOfClass "/Game/Waterline/9_Ocean_Sim_BETA/BP_Waterline_Ocean_Gen_4.BP_Waterline_Ocean_Gen_4_C"))
          (Rendering|Material|SetScalarParameterValueonMaterials (Variables|/Game/Waterline/9_Ocean_Sim_BETA/BP_Waterline_Ocean_Gen_4.BP_Waterline_Ocean_Gen_4_C|GetFFT%20Controller%201 _returnvalue) "Wave Aplitude" (Variables|Default|GetAmplitude%201))
          (Rendering|Material|SetScalarParameterValueonMaterials (Variables|/Game/Waterline/9_Ocean_Sim_BETA/BP_Waterline_Ocean_Gen_4.BP_Waterline_Ocean_Gen_4_C|GetFFT%20Controller%202 _returnvalue) "Wave Aplitude" (Variables|Default|GetAmplitude%202))
          (Rendering|ClearRenderTarget2D "/Game/Waterline/9_Ocean_Sim_BETA/6_Ocean_Baker/RT_Ocean_Bake.RT_Ocean_Bake" "(R=0.000000,G=0.000000,B=1.000000,A=1.000000)")
          (bind (_canvas _size _context) (Rendering|BeginDrawCanvastoRenderTarget "/Game/Waterline/9_Ocean_Sim_BETA/6_Ocean_Baker/RT_Ocean_Bake.RT_Ocean_Bake"))
          (Variables|Default|SetCanvas _canvas)
          (Variables|Default|SetResolution _size)
          (Variables|Default|SetContext _context)
          (bind _output_get_2 (Variables|Default|SetCells%20Per%20Row (/ (.x (Variables|Default|GetResolution)) (Variables|Default|GetFlip%20Res))))
          (Variables|Default|SetFlip%20Cells%20Max (* _output_get_2 _output_get_2)))))
    (:then_1
      ;[1 0 0] Test Time?
      (Utilities|Time|SetTimerbyFunctionName 0 "Capture Ocean" 0.078125 true)
      (Rendering|SceneCapture|CaptureScene (Variables|Default|GetCapture) :!class /Script/Engine.SceneCaptureComponent2D)
      (if (>= (Variables|Default|GetFlip%20Cells%20Current) (Variables|Default|GetFlip%20Cells%20Max))
        (Rendering|EndDrawCanvastoRenderTarget (Variables|Default|GetContext))
        (Class|KismetSystemLibrary|PauseTimer 0 "Capture Ocean")
        (goto _label Reset)
        (else
          (Rendering|BeginDrawCanvastoRenderTarget "/Game/Waterline/9_Ocean_Sim_BETA/6_Ocean_Baker/RT_Ocean_Bake.RT_Ocean_Bake")
          (Variables|Default|SetCurrent%20Column (Math|Float|%(Float) (Variables|Default|GetFlip%20Cells%20Current) (Variables|Default|GetCells%20Per%20Row)))
          (Canvas|DrawTexture :self (Variables|Default|GetCanvas) :RenderTexture "/Game/Waterline/9_Ocean_Sim_BETA/6_Ocean_Baker/Baker_Dev_Mateirals/RT_Baker_Capture.RT_Baker_Capture" :ScreenPosition (Math|Vector2D|MakeVector2D (* (Variables|Default|GetCurrent%20Column) (Variables|Default|GetFlip%20Res)) (* (Variables|Default|GetCurrent%20Row) (Variables|Default|GetFlip%20Res))) :ScreenSize (Math|Vector2D|MakeVector2D _flip_res _flip_res) :CoordinateSize "(X=1.000000,Y=1.000000)" :BlendMode "BLEND_Opaque" :PivotPoint "(X=0.500000,Y=0.500000)")
          ;[1 1 1] Lerp Ocean States
          (Variables|Default|SetCapture%20Ocean%20Time (+ (Variables|Default|GetCapture%20Ocean%20Time) (Math|Float|SafeDivide (Variables|Default|GetCapture%20Length%20%28s%29) (Variables|Default|GetFlip%20Cells%20Max))))
          (Rendering|Material|SetScalarParameterValue "/Game/Waterline/9_Ocean_Sim_BETA/1_BP_Actors/1_Compute_Shaders/1_Spectrum_P_Collection.1_Spectrum_P_Collection" "Time Override" (Variables|Default|GetCapture%20Ocean%20Time) :!class /Script/Engine.KismetMaterialLibrary)
          (bind _returnvalue_2 (Actor|GetActorOfClass "/Game/Waterline/9_Ocean_Sim_BETA/BP_Waterline_Ocean_Gen_4.BP_Waterline_Ocean_Gen_4_C"))
          (Variables|Default|SetAmplitude%201 (- (Variables|Default|GetAmplitude%201) (/ (Variables|Default|GetOcean%20Amplitude) (Variables|Default|GetFlip%20Cells%20Max))))
          (Rendering|Material|SetScalarParameterValueonMaterials (Variables|/Game/Waterline/9_Ocean_Sim_BETA/BP_Waterline_Ocean_Gen_4.BP_Waterline_Ocean_Gen_4_C|GetFFT%20Controller%201 _returnvalue_2) "Wave Aplitude" (Variables|Default|GetAmplitude%201))
          (Variables|Default|SetAmplitude%202 (+ (/ (Variables|Default|GetOcean%20Amplitude) (Variables|Default|GetFlip%20Cells%20Max)) (Variables|Default|GetAmplitude%202)))
          (Rendering|Material|SetScalarParameterValueonMaterials (Variables|/Game/Waterline/9_Ocean_Sim_BETA/BP_Waterline_Ocean_Gen_4.BP_Waterline_Ocean_Gen_4_C|GetFFT%20Controller%202 _returnvalue_2) "Wave Aplitude" (Variables|Default|GetAmplitude%202))
          (bind _result (Math|Float|IncrementFloat (Variables|Default|GetNumber%20of%20Cells%20Rendered))
            (:%20%20
              (Variables|Default|SetNumber%20of%20Cells%20Rendered _result)
              (Math|Float|IncrementFloat (Variables|Default|GetFlip%20Cells%20Current)
                (:%20%20
                  (if (== (Variables|Default|GetCurrent%20Column) (- (Variables|Default|GetCells%20Per%20Row) 1.0))
                    (Math|Float|IncrementFloat (Variables|Default|GetCurrent%20Row))))))))))))

(fn ConstructionScript
  (bind _debug_plane (Variables|Default|GetDebug%20Plane))
  ;[1 1 1] Preview Result Controls
  (Rendering|Material|SetScalarParameterValue "/Game/Waterline/9_Ocean_Sim_BETA/6_Ocean_Baker/Baker_Dev_Mateirals/MPC_Baker.MPC_Baker" "Depth" (Variables|Default|GetDepth) :!class /Script/Engine.KismetMaterialLibrary)
  (Rendering|Material|SetScalarParameterValue "/Game/Waterline/9_Ocean_Sim_BETA/6_Ocean_Baker/Baker_Dev_Mateirals/MPC_Baker.MPC_Baker" "Offset" (Variables|Default|GetOffset) :!class /Script/Engine.KismetMaterialLibrary)
  (Rendering|Material|SetScalarParameterValue "/Game/Waterline/9_Ocean_Sim_BETA/6_Ocean_Baker/Baker_Dev_Mateirals/MPC_Baker.MPC_Baker" "Preview Displacement" (Variables|Default|GetPreview%20Displacement) :!class /Script/Engine.KismetMaterialLibrary)
  (Rendering|Material|SetScalarParameterValue "/Game/Waterline/9_Ocean_Sim_BETA/6_Ocean_Baker/Baker_Dev_Mateirals/MPC_Baker.MPC_Baker" "Preview Speed" (Variables|Default|GetPreview%20Speed) :!class /Script/Engine.KismetMaterialLibrary)
  (Rendering|Material|SetScalarParameterValue "/Game/Waterline/9_Ocean_Sim_BETA/6_Ocean_Baker/Baker_Dev_Mateirals/MPC_Baker.MPC_Baker" "Preview Tile" (Variables|Default|GetPreview%20Tile) :!class /Script/Engine.KismetMaterialLibrary)
  (bind _returnvalue (Actor|GetActorOfClass "/Game/Waterline/9_Ocean_Sim_BETA/BP_Waterline_Ocean_Gen_4.BP_Waterline_Ocean_Gen_4_C"))
  (Variables|/Script/Engine.SceneCaptureComponent2D|SetOrthoWidth (Variables|Default|GetCapture) (+ (Variables|/Game/Waterline/9_Ocean_Sim_BETA/BP_Waterline_Ocean_Gen_4.BP_Waterline_Ocean_Gen_4_C|Get1%20Ocean%20Tile _returnvalue) (* (/ (Variables|/Game/Waterline/9_Ocean_Sim_BETA/BP_Waterline_Ocean_Gen_4.BP_Waterline_Ocean_Gen_4_C|Get1%20Ocean%20Tile _returnvalue) 512.0) 1e+01)))
  (Transformation|SetActorLocation (Math|Vector|MakeVector (* (Variables|/Game/Waterline/9_Ocean_Sim_BETA/BP_Waterline_Ocean_Gen_4.BP_Waterline_Ocean_Gen_4_C|Get1%20Ocean%20Tile _returnvalue) -1.0) (* (Variables|/Game/Waterline/9_Ocean_Sim_BETA/BP_Waterline_Ocean_Gen_4.BP_Waterline_Ocean_Gen_4_C|Get1%20Ocean%20Tile _returnvalue) -1.0) (.z (Transformation|GetActorLocation))) false false)
  ;[1 1 1] Preview Toggle
  (Transformation|SetWorldScale3D (Variables|Default|GetDebug%20Plane) (Math|Conversions|ToVector(Float) (/ (Variables|/Game/Waterline/9_Ocean_Sim_BETA/BP_Waterline_Ocean_Gen_4.BP_Waterline_Ocean_Gen_4_C|Get1%20Ocean%20Tile _returnvalue) 2e+02)))
  (if (Variables|Default|GetPreview%20Result)
    (Rendering|Material|SetMaterial _debug_plane 0 "/Game/Waterline/9_Ocean_Sim_BETA/6_Ocean_Baker/Baker_Dev_Mateirals/M_Baker_Preview.M_Baker_Preview")
    (else
      (Rendering|Material|SetMaterial _debug_plane 0 "/Game/Waterline/9_Ocean_Sim_BETA/6_Ocean_Baker/Baker_Dev_Mateirals/M_Baker_Debug.M_Baker_Debug"))))