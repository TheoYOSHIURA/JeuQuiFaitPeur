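; BP_Water_Exclude is a box volume that turns off the ocean's underwater post process while the player pawn is inside it.
; Box begin and end overlap events toggle UnderwaterPostProcessVolume on the BP_Waterline_Ocean_Gen_3 found in the level.
; A brief delay after BeginPlay checks existing overlaps, covering a player who spawns inside the box.
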(event OnComponentBeginOverlap(Box)
  (params (OverlappedComponent :type Primitive%20Component%20Object%20Reference) (OtherActor :type Actor%20Object%20Reference) (OtherComp :type Primitive%20Component%20Object%20Reference) (OtherBodyIndex :type Integer) (bFromSweep :type Boolean) (SweepResult :type Hit%20Result%20Structure%20%28by%20ref%29))
  (if (== OtherActor (Game|Player|GetPlayerPawn 0))
    (bind _returnvalue (Actor|GetActorOfClass "/Game/Waterline/3_Ocean_Sim_Content/BP_Waterline_Ocean_Gen_3.BP_Waterline_Ocean_Gen_3_C"))
    (Variables|/Script/Engine.PostProcessComponent|SetbEnabled (Variables|/Game/Waterline/3_Ocean_Sim_Content/BP_Waterline_Ocean_Gen_3.BP_Waterline_Ocean_Gen_3_C|GetUnderwater%20Post-Process%20Volume _returnvalue) false)))

(event OnComponentEndOverlap(Box)
  (params (OverlappedComponent :type Primitive%20Component%20Object%20Reference) (OtherActor :type Actor%20Object%20Reference) (OtherComp :type Primitive%20Component%20Object%20Reference) (OtherBodyIndex :type Integer))
  (if (== OtherActor (Game|Player|GetPlayerPawn 0))
    (bind _returnvalue (Actor|GetActorOfClass "/Game/Waterline/3_Ocean_Sim_Content/BP_Waterline_Ocean_Gen_3.BP_Waterline_Ocean_Gen_3_C"))
    (Variables|/Script/Engine.PostProcessComponent|SetbEnabled (Variables|/Game/Waterline/3_Ocean_Sim_Content/BP_Waterline_Ocean_Gen_3.BP_Waterline_Ocean_Gen_3_C|GetUnderwater%20Post-Process%20Volume _returnvalue) true)))

(event EventBeginPlay
  (bind _box (Variables|Default|GetBox))
  (bind _overlappingactors (Collision|GetOverlappingActors _box 0 :!class /Script/Engine.PrimitiveComponent))
  (Utilities|FlowControl|Delay 0.001)
  (if (> (Utilities|Array|Length _overlappingactors) 0)
    (if (Utilities|Array|ContainsItem _overlappingactors (Game|Player|GetPlayerPawn 0))
      (bind _returnvalue (Actor|GetActorOfClass "/Game/Waterline/3_Ocean_Sim_Content/BP_Waterline_Ocean_Gen_3.BP_Waterline_Ocean_Gen_3_C"))
      (Variables|/Script/Engine.PostProcessComponent|SetbEnabled (Variables|/Game/Waterline/3_Ocean_Sim_Content/BP_Waterline_Ocean_Gen_3.BP_Waterline_Ocean_Gen_3_C|GetUnderwater%20Post-Process%20Volume _returnvalue) false))))

(fn ConstructionScript)