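; Shore manager that generates shoreline data for a Waterline ocean or lake and drives its shore wave, foam and breeze materials.
; A scene capture of listed actors feeds ping-pong jump-flood passes that build a distance-field texture.
; That texture or static ones, plus world mapping, go to surface, underwater and post-process materials.
; Modes cover static, trigger-based and timed dynamic updates, the latter texel-snapping to the water's POV sphere.
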(event OnComponentBeginOverlap(TriggerVolume)
  (params (OverlappedComponent :type Primitive%20Component%20Object%20Reference) (OtherActor :type Actor%20Object%20Reference) (OtherComp :type Primitive%20Component%20Object%20Reference) (OtherBodyIndex :type Integer) (bFromSweep :type Boolean) (SweepResult :type Hit%20Result%20Structure%20%28by%20ref%29))
  (bind _mode (Variables|Default|GetMode))
  ;[1 1 1] Broken Trigger
  (if (== OtherComp (Utilities|Array|Get(acopy) (Actor|GetComponentsbyTag (Variables|Default|GetWaterbody) "/Script/Engine.SphereComponent" "Ocean_POV")))
    (if (Utilities|Enum|Equal(Enum) _mode "NewEnumerator1")
      (CallFunction|ForceUpdate)
      (CallFunction|ForceTransfer)
      (elif (Utilities|Enum|Equal(Enum) _mode "NewEnumerator2")
        (CallFunction|ForceUpdate)
        (CallFunction|ForceUpdate)))))

(event Custom|Force%20Update
  (bind _defaultsceneroot (Variables|Default|GetDefaultSceneRoot))
  (bind _resolution (Variables|Default|GetResolution))
  (bind _resolution_2 (Variables|Default|GetResolution))
  (bind _resolution_3 (Variables|Default|GetResolution))
  (bind _rt_jfa_2 (Variables|JFGen|GetRT%20JFA%202))
  (bind _resolution_4 (Variables|Default|GetResolution))
  (bind _waterbody (Variables|Default|GetWaterbody))
  (bind _rt_jfa_1 (Variables|JFGen|GetRT%20JFA%201))
  (bind _process_capture_material (Variables|Default|GetProcess%20Capture%20Material))
  (bind _raw_capture_material (Variables|Default|GetRAW%20Capture%20Material))
  (bind _returnvalue (Transformation|GetWorldScale _defaultsceneroot))
  (bind _returnvalue_2 (Utilities|GetClass _waterbody))
  (bind _returnvalue_3 (== _returnvalue_2 "/Game/Waterline/9_Ocean_Sim_BETA/BP_Waterline_Ocean_Gen_4.BP_Waterline_Ocean_Gen_4_C"))
  ;[1 1 1] Check if Actor Can Function
  (if _returnvalue_3
    (bind _asbp_waterline_ocean_gen_4 (Utilities|Casting|CastToBP_Waterline_Ocean_Gen_4 (Variables|Default|GetWaterbody)))
    (elif (== _returnvalue_2 0)
      (bind _asbp_lake_2 (Utilities|Casting|CastToBP_Lake_2 (Variables|Default|GetWaterbody)))
      (else
        (Development|PrintString (Utilities|String|Append (Utilities|GetDisplayName self) "Shore Manager: NO Waterbody Reference") true true "(R=1.000000,G=0.352237,B=0.000000,A=1.000000)" 5.0))))
  (Rendering|ClearRenderTarget2D (Variables|JFGen|GetRT%20Shore%20Final))
  ;[1 0 0] Temp Explicit FINAL JFA RT (1/2)
  (Rendering|ResizeRenderTarget2D (Variables|JFGen|GetRT%20Shore%20Final) _resolution_2 _resolution_2)
  (Rendering|ClearRenderTarget2D _rt_jfa_1)
  (Rendering|ResizeRenderTarget2D _rt_jfa_1 _resolution_4 _resolution_4)
  (Rendering|ClearRenderTarget2D _rt_jfa_2)
  (Rendering|ResizeRenderTarget2D _rt_jfa_2 _resolution _resolution)
  ;[1 1 1] Scene Capture - Spawn and Place
  (bind _returnvalue_4 (AddComponent|AddSceneCaptureComponent2D false (Math|Transform|MakeTransform "0.000000,0.000000,-5.000000" "-90.000000,-90.000000,0.000000" "1.000000,1.000000,1.000000")))
  (Transformation|SetWorldScale3D _returnvalue_4 "0, 0, 0")
  (Transformation|SetRelativeLocation _returnvalue_4 "0.000000,0.000000,32.000000" false true)
  ;[1 1 1] Scene Capture Render Target Setup
  (bind _output_get (Variables|ShoreCapture|SetRT%20Shore%20Capture "/Game/Waterline/8_Ocean_Shore/Shore_RTs/RT_Shore_Capture.RT_Shore_Capture"))
  (Variables|/Script/Engine.SceneCaptureComponent2D|SetTextureTarget _returnvalue_4 _output_get)
  (Variables|/Script/Engine.SceneCaptureComponent2D|SetOrthoWidth _returnvalue_4 (* (Math|Float|Max(Float) (.x _returnvalue) (.y _returnvalue)) 1e+02))
  (Rendering|ResizeRenderTarget2D (Variables|ShoreCapture|GetRT%20Shore%20Capture) _resolution_3 _resolution_3)
  ;[1 1 1] Scene Capture - Capture Material Setup
  (Variables|/Script/Engine.SceneCaptureComponent2D|SetPostProcessSettings _returnvalue_4 (Utilities|Struct|MakePostProcessSettings (Utilities|Struct|MakeWeightedBlendables (Utilities|Array|MakeArray (Utilities|Struct|MakeWeightedBlendable 1.0 _raw_capture_material)))))
  (Rendering|Material|SetScalarParameterValue _raw_capture_material "Water Level" (+ (.z (Transformation|GetWorldLocation (select _returnvalue_3 (Variables|/Game/Waterline/9_Ocean_Sim_BETA/BP_Waterline_Ocean_Gen_4.BP_Waterline_Ocean_Gen_4_C|GetWaterPlane _asbp_waterline_ocean_gen_4) (Variables|/Game/Waterline/5_Lake/BP_Lake_2.BP_Lake_2_C|GetWaterPlane _asbp_lake_2)))) (Variables|Default|GetOffset%20Water%20Level)) :!class /Script/Engine.MaterialInstanceDynamic)
  (Rendering|Material|SetScalarParameterValue _raw_capture_material "Bit Mask" (Variables|Default|GetBlock%20Shore%20Stencil) :!class /Script/Engine.MaterialInstanceDynamic)
  ;[1 1 1] Transfer Capture to Shore Pass
  (Rendering|Material|SetScalarParameterValue (Variables|Default|GetProcess%20Capture%20Material) "Shore Offset" (Variables|Default|GetShore%20Offset) :!class /Script/Engine.MaterialInstanceDynamic)
  ;[1 1 1] Scene Capture Show ONLY List
  (for _array_element (Variables|ShoreCapture|GetCapture%20Actors)
    (Rendering|SceneCapture|ShowOnlyActorComponents _returnvalue_4 _array_element false))
  (if (Variables|Default|GetShore%20Warmup)
    _
    (else
      (Utilities|FlowControl|Delay 1.0)
      (Variables|Default|SetShore%20Warmup true)))
  ;[1 0.4428 0] Scene Capture Trigger
  (Rendering|SceneCapture|CaptureScene _returnvalue_4 :!class /Script/Engine.SceneCaptureComponent2D)
  (Rendering|Material|SetTextureParameterValue (Variables|Default|GetProcess%20Capture%20Material) "Shore Capture RAW" "/Game/Waterline/8_Ocean_Shore/Shore_RTs/RT_Shore_Capture.RT_Shore_Capture")
  ;[1 1 1] JFA Render
  (for _index (range 0 (Math|Float|Truncate (/ (Math|Float|Loge (Math|Conversions|ToFloat(Integer) (Variables|Default|GetResolution))) (Math|Float|Loge 2.0))))
    (Utilities|FlowControl|FlipFlop
      (:A
        (bind (_canvas _size _context) (Rendering|BeginDrawCanvastoRenderTarget (Variables|JFGen|GetRT%20JFA%201)))
        (Canvas|DrawMaterial :self _canvas :RenderMaterial _process_capture_material :ScreenSize _size :CoordinateSize "(X=1.000000,Y=1.000000)" :PivotPoint "(X=0.500000,Y=0.500000)")
        (Rendering|EndDrawCanvastoRenderTarget _context)
        (Rendering|Material|SetTextureParameterValue _process_capture_material "Shore Capture RAW" (Variables|JFGen|GetRT%20JFA%201)))
      (:B
        (bind (_canvas_2 _size_2 _context_2) (Rendering|BeginDrawCanvastoRenderTarget (Variables|JFGen|GetRT%20JFA%202)))
        (Canvas|DrawMaterial :self _canvas_2 :RenderMaterial _process_capture_material :ScreenSize _size_2 :CoordinateSize "(X=1.000000,Y=1.000000)" :PivotPoint "(X=0.500000,Y=0.500000)")
        (Rendering|EndDrawCanvastoRenderTarget _context_2)
        (Rendering|Material|SetTextureParameterValue _process_capture_material "Shore Capture RAW" (Variables|JFGen|GetRT%20JFA%202)))))
  ;[1 0 0] Temp Explicit FINAL JFA RT (2/2)
  (Rendering|DrawMaterialtoRenderTarget (Variables|JFGen|GetRT%20Shore%20Final) _process_capture_material)
  (CallFunction|ForceTransfer))

(event Custom|Force%20Transfer
  (bind _waterbody (Variables|Default|GetWaterbody))
  (bind _waterbody_2 (Variables|Default|GetWaterbody))
  (bind _mode (Variables|Default|GetMode))
  (bind _defaultsceneroot (Variables|Default|GetDefaultSceneRoot))
  (bind _returnvalue (Transformation|GetWorldScale _defaultsceneroot))
  (bind _returnvalue_2 (Utilities|GetClass _waterbody_2))
  (bind _returnvalue_3 (== _returnvalue_2 "/Game/Waterline/9_Ocean_Sim_BETA/BP_Waterline_Ocean_Gen_4.BP_Waterline_Ocean_Gen_4_C"))
  ;[1 1 1] Send Texture Data to Waterline Actor
  (if (Utilities|Enum|Equal(Enum) (Variables|Default|GetMode) "NewEnumerator3")
    (Utilities|Time|SetTimerbyEvent (delegate Custom|Force%20Transfer) (/ 1.0 (Math|Float|SelectFloat (Variables|Default|GetShore%20Generation%20Framerate) 3e+01 (Variables|Default|GetShore%20Warmup))) true)
    (else
      (Class|KismetSystemLibrary|PauseTimer 0 "Force Transfer")))
  (if _returnvalue_3
    (bind _asbp_waterline_ocean_gen_4 (Utilities|Casting|CastToBP_Waterline_Ocean_Gen_4 _waterbody))
    ;[1 1 1] Shore RAW Capture Transformation for Material WS Mapping
    (Rendering|Material|SetScalarParameterValue (select _returnvalue_3 (Variables|/Game/Waterline/9_Ocean_Sim_BETA/BP_Waterline_Ocean_Gen_4.BP_Waterline_Ocean_Gen_4_C|GetWater%20Surface%20DYN _asbp_waterline_ocean_gen_4) (Variables|/Game/Waterline/5_Lake/BP_Lake_2.BP_Lake_2_C|GetWater%20Surface%20DYN (stale _asbp_lake_2))) "Shore Texture Scale" (* (Math|Float|Max(Float) (.x _returnvalue) (.y _returnvalue)) 1e+02) :!class /Script/Engine.MaterialInstanceDynamic :!label _label)
    (Rendering|Material|SetScalarParameterValue (select _returnvalue_3 (Variables|/Game/Waterline/9_Ocean_Sim_BETA/BP_Waterline_Ocean_Gen_4.BP_Waterline_Ocean_Gen_4_C|GetWater%20Surface%20DYN _asbp_waterline_ocean_gen_4) (Variables|/Game/Waterline/5_Lake/BP_Lake_2.BP_Lake_2_C|GetWater%20Surface%20DYN (stale _asbp_lake_2))) "Shore Texture Angle" (.yaw (Transformation|GetWorldRotation (Variables|Default|GetDefaultSceneRoot))) :!class /Script/Engine.MaterialInstanceDynamic)
    (Rendering|Material|SetVectorParameterValue (select _returnvalue_3 (Variables|/Game/Waterline/9_Ocean_Sim_BETA/BP_Waterline_Ocean_Gen_4.BP_Waterline_Ocean_Gen_4_C|GetWater%20Surface%20DYN _asbp_waterline_ocean_gen_4) (Variables|/Game/Waterline/5_Lake/BP_Lake_2.BP_Lake_2_C|GetWater%20Surface%20DYN (stale _asbp_lake_2))) "Shore Texture Location" (Math|Conversions|ToLinearColor(Vector) (Transformation|GetWorldLocation (Variables|Default|GetDefaultSceneRoot))) :!class /Script/Engine.MaterialInstanceDynamic)
    ;[1 1 1] Shore Texture Data Set
    (if (or (Utilities|Enum|Equal(Enum) _mode "NewEnumerator1") (Utilities|Enum|Equal(Enum) _mode "NewEnumerator0"))
      (Rendering|Material|SetTextureParameterValue (select _returnvalue_3 (Variables|/Game/Waterline/9_Ocean_Sim_BETA/BP_Waterline_Ocean_Gen_4.BP_Waterline_Ocean_Gen_4_C|GetWater%20Surface%20DYN _asbp_waterline_ocean_gen_4) (Variables|/Game/Waterline/5_Lake/BP_Lake_2.BP_Lake_2_C|GetWater%20Surface%20DYN (stale _asbp_lake_2))) "Shore Data Texture" (Variables|StaticAssets|GetStatic%20Shore))
      (Rendering|Material|SetTextureParameterValue (select _returnvalue_3 (Variables|/Game/Waterline/9_Ocean_Sim_BETA/BP_Waterline_Ocean_Gen_4.BP_Waterline_Ocean_Gen_4_C|GetWater%20Surface%20DYN _asbp_waterline_ocean_gen_4) (Variables|/Game/Waterline/5_Lake/BP_Lake_2.BP_Lake_2_C|GetWater%20Surface%20DYN (stale _asbp_lake_2))) "Shore Capture Texture" (Variables|StaticAssets|GetStatic%20Capture))
      (else
        (Rendering|Material|SetTextureParameterValue (select _returnvalue_3 (Variables|/Game/Waterline/9_Ocean_Sim_BETA/BP_Waterline_Ocean_Gen_4.BP_Waterline_Ocean_Gen_4_C|GetWater%20Surface%20DYN _asbp_waterline_ocean_gen_4) (Variables|/Game/Waterline/5_Lake/BP_Lake_2.BP_Lake_2_C|GetWater%20Surface%20DYN (stale _asbp_lake_2))) "Shore Data Texture" (Variables|JFGen|GetRT%20Shore%20Final))
        (Rendering|Material|SetTextureParameterValue (select _returnvalue_3 (Variables|/Game/Waterline/9_Ocean_Sim_BETA/BP_Waterline_Ocean_Gen_4.BP_Waterline_Ocean_Gen_4_C|GetWater%20Surface%20DYN _asbp_waterline_ocean_gen_4) (Variables|/Game/Waterline/5_Lake/BP_Lake_2.BP_Lake_2_C|GetWater%20Surface%20DYN (stale _asbp_lake_2))) "Shore Capture Texture" (Variables|ShoreCapture|GetRT%20Shore%20Capture))))
    (CallFunction|ShoreMaterialProperties (select _returnvalue_3 (Variables|/Game/Waterline/9_Ocean_Sim_BETA/BP_Waterline_Ocean_Gen_4.BP_Waterline_Ocean_Gen_4_C|GetWater%20Surface%20DYN _asbp_waterline_ocean_gen_4) (Variables|/Game/Waterline/5_Lake/BP_Lake_2.BP_Lake_2_C|GetWater%20Surface%20DYN (stale _asbp_lake_2))) (select (Variables|/Game/Waterline/9_Ocean_Sim_BETA/BP_Waterline_Ocean_Gen_4.BP_Waterline_Ocean_Gen_4_C|GetUnderwater%20Surface%20Enable _asbp_waterline_ocean_gen_4) (select _returnvalue_3 (Variables|/Game/Waterline/9_Ocean_Sim_BETA/BP_Waterline_Ocean_Gen_4.BP_Waterline_Ocean_Gen_4_C|GetUnderwater%20Surface%20DYN _asbp_waterline_ocean_gen_4) (Variables|/Game/Waterline/5_Lake/BP_Lake_2.BP_Lake_2_C|GetUnderwater%20Surface%20DYN (stale _asbp_lake_2))) (select _returnvalue_3 (Variables|/Game/Waterline/9_Ocean_Sim_BETA/BP_Waterline_Ocean_Gen_4.BP_Waterline_Ocean_Gen_4_C|GetWater%20Surface%20DYN _asbp_waterline_ocean_gen_4) (Variables|/Game/Waterline/5_Lake/BP_Lake_2.BP_Lake_2_C|GetWater%20Surface%20DYN (stale _asbp_lake_2)))) (select _returnvalue_3 (Variables|/Game/Waterline/9_Ocean_Sim_BETA/BP_Waterline_Ocean_Gen_4.BP_Waterline_Ocean_Gen_4_C|GetPost-Process%20DYN _asbp_waterline_ocean_gen_4) (Variables|/Game/Waterline/5_Lake/BP_Lake_2.BP_Lake_2_C|GetPost-Process%20DYN (stale _asbp_lake_2))))
    (elif (== _returnvalue_2 "/Game/Waterline/5_Lake/BP_Lake_2.BP_Lake_2_C")
      (bind _asbp_lake_2 (Utilities|Casting|CastToBP_Lake_2 _waterbody))
      (goto _label))))

(event Custom|Full%20Dynamic%20Gen
  (bind _process_capture_material (Variables|Default|GetProcess%20Capture%20Material))
  (Utilities|Time|SetTimerbyEvent (delegate Custom|Full%20Dynamic%20Gen) (/ 1.0 (Variables|Default|GetShore%20Generation%20Framerate)) true)
  (Transformation|SetActorLocation (* (+ (Math|Vector|MakeVector (Math|Conversions|ToFloat(Integer) (Math|Float|Floor (.x (/ (Transformation|GetWorldLocation (Utilities|Array|Get(acopy) (Actor|GetComponentsbyTag (Variables|Default|GetWaterbody) "/Script/Engine.SphereComponent" "Ocean_POV"))) (* (/ 1.0 (Math|Conversions|ToFloat(Integer) (Variables|Default|GetResolution))) (Variables|/Script/Engine.SceneCaptureComponent2D|GetOrthoWidth (stale Custom|Force%20Update _returnvalue_4))))))) (Math|Conversions|ToFloat(Integer) (Math|Float|Floor (.y (/ (Transformation|GetWorldLocation (Utilities|Array|Get(acopy) (Actor|GetComponentsbyTag (Variables|Default|GetWaterbody) "/Script/Engine.SphereComponent" "Ocean_POV"))) (* (/ 1.0 (Math|Conversions|ToFloat(Integer) (Variables|Default|GetResolution))) (Variables|/Script/Engine.SceneCaptureComponent2D|GetOrthoWidth (stale Custom|Force%20Update _returnvalue_4))))))) (Math|Conversions|ToFloat(Integer) (Math|Float|Floor (.z (/ (Transformation|GetWorldLocation (Utilities|Array|Get(acopy) (Actor|GetComponentsbyTag (Variables|Default|GetWaterbody) "/Script/Engine.SphereComponent" "Ocean_POV"))) (* (/ 1.0 (Math|Conversions|ToFloat(Integer) (Variables|Default|GetResolution))) (Variables|/Script/Engine.SceneCaptureComponent2D|GetOrthoWidth (stale Custom|Force%20Update _returnvalue_4)))))))) 0.5) (* (/ 1.0 (Math|Conversions|ToFloat(Integer) (Variables|Default|GetResolution))) (Variables|/Script/Engine.SceneCaptureComponent2D|GetOrthoWidth (stale Custom|Force%20Update _returnvalue_4)))) false false)
  ;[1 1 1] Transfer Capture to Shore Pass
  (Rendering|Material|SetScalarParameterValue (Variables|Default|GetProcess%20Capture%20Material) "Shore Offset" (Variables|Default|GetShore%20Offset) :!class /Script/Engine.MaterialInstanceDynamic)
  ;[1 1 1] Scene Capture Show ONLY List
  (for _array_element (Variables|ShoreCapture|GetCapture%20Actors)
    (Rendering|SceneCapture|ShowOnlyActorComponents (stale Custom|Force%20Update _returnvalue_4) _array_element false))
  (if (Variables|Default|GetShore%20Warmup)
    _
    (else
      (Utilities|FlowControl|Delay 1.0)
      (Variables|Default|SetShore%20Warmup true)))
  ;[1 0.4428 0] Scene Capture Trigger
  (Rendering|SceneCapture|CaptureScene (stale Custom|Force%20Update _returnvalue_4) :!class /Script/Engine.SceneCaptureComponent2D)
  (Rendering|Material|SetTextureParameterValue (Variables|Default|GetProcess%20Capture%20Material) "Shore Capture RAW" "/Game/Waterline/8_Ocean_Shore/Shore_RTs/RT_Shore_Capture.RT_Shore_Capture")
  ;[1 1 1] JFA Render
  (for _index (range 0 (Math|Float|Truncate (/ (Math|Float|Loge (Math|Conversions|ToFloat(Integer) (Variables|Default|GetResolution))) (Math|Float|Loge 2.0))))
    (Utilities|FlowControl|FlipFlop
      (:A
        (bind (_canvas _size _context) (Rendering|BeginDrawCanvastoRenderTarget (Variables|JFGen|GetRT%20JFA%201)))
        (Canvas|DrawMaterial :self _canvas :RenderMaterial _process_capture_material :ScreenSize _size :CoordinateSize "(X=1.000000,Y=1.000000)" :PivotPoint "(X=0.500000,Y=0.500000)")
        (Rendering|EndDrawCanvastoRenderTarget _context)
        (Rendering|Material|SetTextureParameterValue _process_capture_material "Shore Capture RAW" (Variables|JFGen|GetRT%20JFA%201)))
      (:B
        (bind (_canvas_2 _size_2 _context_2) (Rendering|BeginDrawCanvastoRenderTarget (Variables|JFGen|GetRT%20JFA%202)))
        (Canvas|DrawMaterial :self _canvas_2 :RenderMaterial _process_capture_material :ScreenSize _size_2 :CoordinateSize "(X=1.000000,Y=1.000000)" :PivotPoint "(X=0.500000,Y=0.500000)")
        (Rendering|EndDrawCanvastoRenderTarget _context_2)
        (Rendering|Material|SetTextureParameterValue _process_capture_material "Shore Capture RAW" (Variables|JFGen|GetRT%20JFA%202)))))
  ;[1 0 0] Temp Explicit FINAL JFA RT (2/2)
  (Rendering|DrawMaterialtoRenderTarget (Variables|JFGen|GetRT%20Shore%20Final) _process_capture_material)
  (CallFunction|ForceTransfer))

(event EventBeginPlay
  (bind _mode (Variables|Default|GetMode))
  (bind _mode_2 (Variables|Default|GetMode))
  (Variables|Default|SetShore%20Warmup false)
  (if (Utilities|Enum|Equal(Enum) (Variables|Default|GetMode) "NewEnumerator3")
    (CallFunction|ForceUpdate)
    (CallFunction|FullDynamicGen)
    (else
      ;[1 1 1] Broken Trigger
      (if (or (Utilities|Enum|Equal(Enum) _mode_2 "NewEnumerator1") (Utilities|Enum|Equal(Enum) _mode_2 "NewEnumerator2"))
        (if (Class|PrimitiveComponent|IsOverlappingComponent (Variables|Default|GetTrigger%20Volume) (Utilities|Array|Get(acopy) (Actor|GetComponentsbyTag (Variables|Default|GetWaterbody) "/Script/Engine.SphereComponent" "Ocean_POV")))
          (if (Utilities|Enum|Equal(Enum) _mode "NewEnumerator1")
            (CallFunction|ForceUpdate)
            (CallFunction|ForceTransfer :!label _label)
            (elif (Utilities|Enum|Equal(Enum) _mode "NewEnumerator2")
              (CallFunction|ForceUpdate)
              (CallFunction|ForceUpdate))))
        (else
          (goto _label))))))

(fn ConstructionScript
  (bind _capture_size (Variables|Default|GetCapture%20Size))
  (bind _mode (Variables|Default|GetMode))
  (bind _trigger_volume (Variables|Default|GetTrigger%20Volume))
  (bind _waterbody (Variables|Default|GetWaterbody))
  (bind _waterbody_2 (Variables|Default|GetWaterbody))
  (bind _defaultsceneroot (Variables|Default|GetDefaultSceneRoot))
  (bind _returnvalue (Transformation|GetWorldScale _defaultsceneroot))
  (bind _returnvalue_2 (Utilities|GetClass _waterbody_2))
  (bind _returnvalue_3 (Utilities|GetClass _waterbody))
  (bind _returnvalue_4 (== _returnvalue_2 "/Game/Waterline/9_Ocean_Sim_BETA/BP_Waterline_Ocean_Gen_4.BP_Waterline_Ocean_Gen_4_C"))
  (Class|BoxComponent|SetLineThickness (Variables|Default|GetCapture%20Volume) (Variables|Default|GetLine%20Thickness))
  (Rendering|SetVisibility (Variables|Default|GetDebug%20Canvas) (Variables|Default|GetView%20Debug%20Texture) false)
  (Transformation|SetActorScale3D (Math|Vector|MakeVector _capture_size _capture_size 4e+02))
  (Transformation|SetActorRotation "0, 0, 0")
  (Components|Box|SetBoxExtent _trigger_volume (Variables|Default|GetTrigger%20Volume%20Extent) true)
  (bind _returnvalue_5 (Rendering|Material|CreateDynamicMaterialInstance "/Game/Waterline/8_Ocean_Shore/Shore_Gen_Mat/M_Capture_Depth.M_Capture_Depth" "None" "None" :!class /Script/Engine.KismetMaterialLibrary))
  (Variables|Default|SetRAW%20Capture%20Material _returnvalue_5)
  (bind _returnvalue_6 (Rendering|Material|CreateDynamicMaterialInstance "/Game/Waterline/8_Ocean_Shore/Shore_Gen_Mat/M_DF_Shore_Gen_V2.M_DF_Shore_Gen_V2" "None" "None" :!class /Script/Engine.KismetMaterialLibrary))
  (Variables|Default|SetProcess%20Capture%20Material _returnvalue_6)
  (Variables|/Script/Engine.PrimitiveComponent|SetbGenerateOverlapEvents _trigger_volume (or (Utilities|Enum|Equal(Enum) _mode "NewEnumerator1") (Utilities|Enum|Equal(Enum) _mode "NewEnumerator2")))
  ;[1 1 1] Material Edit in Editor
  (if (== _returnvalue_3 "/Game/Waterline/9_Ocean_Sim_BETA/BP_Waterline_Ocean_Gen_4.BP_Waterline_Ocean_Gen_4_C")
    (bind _asbp_waterline_ocean_gen_4 (Utilities|Casting|CastToBP_Waterline_Ocean_Gen_4 (Variables|Default|GetWaterbody)))
    ;[1 1 1] Shore RAW Capture Transformation for Material WS Mapping
    (Rendering|Material|SetTextureParameterValue (select _returnvalue_4 (Variables|/Game/Waterline/9_Ocean_Sim_BETA/BP_Waterline_Ocean_Gen_4.BP_Waterline_Ocean_Gen_4_C|GetWater%20Surface%20DYN _asbp_waterline_ocean_gen_4) (Variables|/Game/Waterline/5_Lake/BP_Lake_2.BP_Lake_2_C|GetWater%20Surface%20DYN (stale _asbp_lake_2))) "Shore Data Texture" (Variables|JFGen|GetRT%20Shore%20Final) :!label _label)
    (Rendering|Material|SetScalarParameterValue (select _returnvalue_4 (Variables|/Game/Waterline/9_Ocean_Sim_BETA/BP_Waterline_Ocean_Gen_4.BP_Waterline_Ocean_Gen_4_C|GetWater%20Surface%20DYN _asbp_waterline_ocean_gen_4) (Variables|/Game/Waterline/5_Lake/BP_Lake_2.BP_Lake_2_C|GetWater%20Surface%20DYN (stale _asbp_lake_2))) "Shore Texture Scale" (* (Math|Float|Max(Float) (.x _returnvalue) (.y _returnvalue)) 1e+02) :!class /Script/Engine.MaterialInstanceDynamic)
    (Rendering|Material|SetScalarParameterValue (select _returnvalue_4 (Variables|/Game/Waterline/9_Ocean_Sim_BETA/BP_Waterline_Ocean_Gen_4.BP_Waterline_Ocean_Gen_4_C|GetWater%20Surface%20DYN _asbp_waterline_ocean_gen_4) (Variables|/Game/Waterline/5_Lake/BP_Lake_2.BP_Lake_2_C|GetWater%20Surface%20DYN (stale _asbp_lake_2))) "Shore Texture Angle" (.yaw (Transformation|GetWorldRotation (Variables|Default|GetDefaultSceneRoot))) :!class /Script/Engine.MaterialInstanceDynamic)
    (Rendering|Material|SetVectorParameterValue (select _returnvalue_4 (Variables|/Game/Waterline/9_Ocean_Sim_BETA/BP_Waterline_Ocean_Gen_4.BP_Waterline_Ocean_Gen_4_C|GetWater%20Surface%20DYN _asbp_waterline_ocean_gen_4) (Variables|/Game/Waterline/5_Lake/BP_Lake_2.BP_Lake_2_C|GetWater%20Surface%20DYN (stale _asbp_lake_2))) "Shore Texture Location" (Math|Conversions|ToLinearColor(Vector) (Transformation|GetWorldLocation (Variables|Default|GetDefaultSceneRoot))) :!class /Script/Engine.MaterialInstanceDynamic)
    (CallFunction|ShoreMaterialProperties (select _returnvalue_4 (Variables|/Game/Waterline/9_Ocean_Sim_BETA/BP_Waterline_Ocean_Gen_4.BP_Waterline_Ocean_Gen_4_C|GetWater%20Surface%20DYN _asbp_waterline_ocean_gen_4) (Variables|/Game/Waterline/5_Lake/BP_Lake_2.BP_Lake_2_C|GetWater%20Surface%20DYN (stale _asbp_lake_2))) (select (Variables|/Game/Waterline/9_Ocean_Sim_BETA/BP_Waterline_Ocean_Gen_4.BP_Waterline_Ocean_Gen_4_C|GetUnderwater%20Surface%20Enable _asbp_waterline_ocean_gen_4) (select _returnvalue_4 (Variables|/Game/Waterline/9_Ocean_Sim_BETA/BP_Waterline_Ocean_Gen_4.BP_Waterline_Ocean_Gen_4_C|GetUnderwater%20Surface%20DYN _asbp_waterline_ocean_gen_4) (Variables|/Game/Waterline/5_Lake/BP_Lake_2.BP_Lake_2_C|GetUnderwater%20Surface%20DYN (stale _asbp_lake_2))) (select _returnvalue_4 (Variables|/Game/Waterline/9_Ocean_Sim_BETA/BP_Waterline_Ocean_Gen_4.BP_Waterline_Ocean_Gen_4_C|GetWater%20Surface%20DYN _asbp_waterline_ocean_gen_4) (Variables|/Game/Waterline/5_Lake/BP_Lake_2.BP_Lake_2_C|GetWater%20Surface%20DYN (stale _asbp_lake_2)))) (select _returnvalue_4 (Variables|/Game/Waterline/9_Ocean_Sim_BETA/BP_Waterline_Ocean_Gen_4.BP_Waterline_Ocean_Gen_4_C|GetPost-Process%20DYN _asbp_waterline_ocean_gen_4) (Variables|/Game/Waterline/5_Lake/BP_Lake_2.BP_Lake_2_C|GetPost-Process%20DYN (stale _asbp_lake_2))))
    (elif (== _returnvalue_3 0)
      (bind _asbp_lake_2 (Utilities|Casting|CastToBP_Lake_2 (Variables|Default|GetWaterbody)))
      (goto _label))))

(fn ShoreMaterialProperties
  (params (Water%20Material :type Material%20Instance%20Dynamic%20Object%20Reference) (Underwater%20Surface%20Material :type Material%20Instance%20Dynamic%20Object%20Reference) (Underwater%20VFX%20Material :type Material%20Instance%20Dynamic%20Object%20Reference))
  (Utilities|FlowControl|Sequence
    (:then_0
      (Rendering|Material|SetScalarParameterValue Water%20Material "Shore Wave Animation Speed" (Variables|ShoreParameters|GetShore%20Wave%20Animation%20Speed) :!class /Script/Engine.MaterialInstanceDynamic)
      (Rendering|Material|SetScalarParameterValue Water%20Material "Shore Wave Deep Clamp" (Variables|ShoreParameters|GetShore%20Wave%20Deep%20Clamp) :!class /Script/Engine.MaterialInstanceDynamic)
      (Rendering|Material|SetVectorParameterValue Water%20Material "Shore Wave Displacement" (Math|Conversions|ToLinearColor(Vector) (Variables|ShoreParameters|GetShore%20Wave%20Displacement)) :!class /Script/Engine.MaterialInstanceDynamic)
      (Rendering|Material|SetScalarParameterValue Water%20Material "Shore Wave Distortion" (Variables|ShoreParameters|GetShore%20Wave%20Distortion) :!class /Script/Engine.MaterialInstanceDynamic)
      (Rendering|Material|SetScalarParameterValue Water%20Material "Shore Wave Normal Power" (Variables|ShoreParameters|GetShore%20Wave%20Normal%20Power) :!class /Script/Engine.MaterialInstanceDynamic)
      (Rendering|Material|SetScalarParameterValue Water%20Material "Shore Wave Normal Texel Size" (Variables|ShoreParameters|GetShore%20Wave%20Normal%20Texel%20Size) :!class /Script/Engine.MaterialInstanceDynamic)
      (Rendering|Material|SetScalarParameterValue Water%20Material "Shore Wave Offset" (Variables|ShoreParameters|GetShore%20Wave%20Offset) :!class /Script/Engine.MaterialInstanceDynamic)
      (Rendering|Material|SetScalarParameterValue Water%20Material "Shore Wave Panning Speed" (Variables|ShoreParameters|GetShore%20Wave%20Panning%20Speed) :!class /Script/Engine.MaterialInstanceDynamic)
      (Rendering|Material|SetScalarParameterValue Water%20Material "Shore Wave Shallow Blend" (Variables|ShoreParameters|GetShore%20Wave%20Shallow%20Blend) :!class /Script/Engine.MaterialInstanceDynamic)
      (Rendering|Material|SetScalarParameterValue Water%20Material "Shore Wave Shallow Clamp" (Variables|ShoreParameters|GetShore%20Wave%20Shallow%20Clamp) :!class /Script/Engine.MaterialInstanceDynamic)
      (Rendering|Material|SetScalarParameterValue Water%20Material "Shore Wave Soften Normal" (Variables|ShoreParameters|GetShore%20Wave%20Soften%20Normal) :!class /Script/Engine.MaterialInstanceDynamic)
      (Rendering|Material|SetTextureParameterValue Water%20Material "Shore Wave Texture" (Variables|ShoreParameters|GetShore%20Wave%20Texture))
      (Rendering|Material|SetVectorParameterValue Water%20Material "Shore Wave Tiling" (Math|Conversions|ToLinearColor(Vector) (Variables|ShoreParameters|GetShore%20Wave%20Tiling)) :!class /Script/Engine.MaterialInstanceDynamic)
      (Rendering|Material|SetScalarParameterValue Water%20Material "Shore Wind Direction" (Variables|ShoreParameters|GetShore%20Wind%20Direction) :!class /Script/Engine.MaterialInstanceDynamic)
      (Rendering|Material|SetScalarParameterValue Water%20Material "Shore Wind Direction Influence" (Variables|ShoreParameters|GetShore%20Wind%20Direction%20Influence) :!class /Script/Engine.MaterialInstanceDynamic)
      (Rendering|Material|SetTextureParameterValue Water%20Material "Shore Wave Normal Texture" (Variables|ShoreParameters|GetShore%20Wave%20Normal%20Texture))
      (Rendering|Material|SetTextureParameterValue Water%20Material "Shore Wave Texture" (Variables|ShoreParameters|GetShore%20Wave%20Texture))
      (Rendering|Material|SetTextureParameterValue Water%20Material "Shore Wave Foam Texture" (Variables|ShoreParameters|GetShore%20Wave%20Foam%20Texture)))
    (:then_1
      (Rendering|Material|SetScalarParameterValue Water%20Material "Shore Shallows Blend" (Variables|ShoreParameters|GetShore%20Shallows%20Blend) :!class /Script/Engine.MaterialInstanceDynamic)
      (Rendering|Material|SetScalarParameterValue Water%20Material "Shore Shallows Range" (Variables|ShoreParameters|GetShore%20Shallows%20Range) :!class /Script/Engine.MaterialInstanceDynamic))
    (:then_2
      (Rendering|Material|SetScalarParameterValue Water%20Material "Shore Normal MAX Blend" (Variables|ShoreParameters|GetShore%20Normal%20MAX%20Blend) :!class /Script/Engine.MaterialInstanceDynamic)
      (Rendering|Material|SetScalarParameterValue Water%20Material "Shore Normal MIN Blend" (Variables|ShoreParameters|GetShore%20Normal%20MIN%20Blend) :!class /Script/Engine.MaterialInstanceDynamic)
      (Rendering|Material|SetScalarParameterValue Water%20Material "Shore Normal MIN Shift" (Variables|ShoreParameters|GetShore%20Normal%20Shift) :!class /Script/Engine.MaterialInstanceDynamic))
    (:then_3
      (Rendering|Material|SetScalarParameterValue Water%20Material "Shore Noise Contrast" (Variables|ShoreParameters|GetShore%20Noise%20Contrast) :!class /Script/Engine.MaterialInstanceDynamic)
      (Rendering|Material|SetScalarParameterValue Water%20Material "Shore Noise Power" (Variables|ShoreParameters|GetShore%20Noise%20Power) :!class /Script/Engine.MaterialInstanceDynamic)
      (Rendering|Material|SetScalarParameterValue Water%20Material "Shore Noise Scale" (Variables|ShoreParameters|GetShore%20Noise%20Scale) :!class /Script/Engine.MaterialInstanceDynamic)
      (Rendering|Material|SetTextureParameterValue Water%20Material "Shore Noise Texture" (Variables|ShoreParameters|GetShore%20Noise%20Texture)))
    (:then_4
      (Rendering|Material|SetScalarParameterValue Water%20Material "Shore Foam Blend" (Variables|ShoreParameters|GetShore%20Foam%20Blend) :!class /Script/Engine.MaterialInstanceDynamic)
      (Rendering|Material|SetScalarParameterValue Water%20Material "Shore Foam MIN Blend" (Variables|ShoreParameters|GetShore%20Foam%20MIN%20Blend) :!class /Script/Engine.MaterialInstanceDynamic)
      (Rendering|Material|SetScalarParameterValue Water%20Material "Shore Foam MIN Shift" (Variables|ShoreParameters|GetShore%20Foam%20MIN%20Shift) :!class /Script/Engine.MaterialInstanceDynamic)
      (Rendering|Material|SetScalarParameterValue Water%20Material "Shore Foam Offset" (Variables|ShoreParameters|GetShore%20Foam%20Offset) :!class /Script/Engine.MaterialInstanceDynamic)
      (Rendering|Material|SetScalarParameterValue Water%20Material "Shore Foam Power" (Variables|ShoreParameters|GetShore%20Foam%20Power) :!class /Script/Engine.MaterialInstanceDynamic))
    (:then_5
      (Rendering|Material|SetScalarParameterValue Water%20Material "Grav Foam" (Variables|ShoreParameters|GetGrav%20Foam) :!class /Script/Engine.MaterialInstanceDynamic)
      (Rendering|Material|SetScalarParameterValue Water%20Material "Grav Level" (Variables|ShoreParameters|GetGrav%20Level) :!class /Script/Engine.MaterialInstanceDynamic)
      (Rendering|Material|SetScalarParameterValue Water%20Material "Grav Level Blend" (Variables|ShoreParameters|GetGrav%20Level%20Blend) :!class /Script/Engine.MaterialInstanceDynamic)
      (Rendering|Material|SetScalarParameterValue Water%20Material "Grav Speed" (Variables|ShoreParameters|GetGrav%20Speed) :!class /Script/Engine.MaterialInstanceDynamic)
      (Rendering|Material|SetScalarParameterValue Water%20Material "Grav Wave Climb" (Variables|ShoreParameters|GetGrav%20Wave%20Climb) :!class /Script/Engine.MaterialInstanceDynamic)
      (Rendering|Material|SetScalarParameterValue Water%20Material "Grav Flow" (Variables|ShoreParameters|GetGrav%20Wave%20Flow) :!class /Script/Engine.MaterialInstanceDynamic))
    (:then_6
      (Rendering|Material|SetTextureParameterValue Water%20Material "Breeze Texture" (Variables|ShoreParameters|GetBreeze%20Texture))
      (Rendering|Material|SetVectorParameterValue Water%20Material "Breeze Texture Scale" (Math|Conversions|ToLinearColor(Vector) (Variables|ShoreParameters|GetBreeze%20Texture%20Scale)) :!class /Script/Engine.MaterialInstanceDynamic)
      (Rendering|Material|SetScalarParameterValue Water%20Material "Breeze Texture Soften" (Variables|ShoreParameters|GetBreeze%20Texture%20Soften) :!class /Script/Engine.MaterialInstanceDynamic)
      (Rendering|Material|SetScalarParameterValue Water%20Material "Breeze Animation Distort" (Variables|ShoreParameters|GetBreeze%20Animation%20Distort) :!class /Script/Engine.MaterialInstanceDynamic)
      (Rendering|Material|SetScalarParameterValue Water%20Material "Breeze Animation Speed" (Variables|ShoreParameters|GetBreeze%20Animation%20Speed) :!class /Script/Engine.MaterialInstanceDynamic)
      (Rendering|Material|SetScalarParameterValue Water%20Material "Breeze Exclude Mask" (Variables|ShoreParameters|GetBreeze%20Exclude%20Mask) :!class /Script/Engine.MaterialInstanceDynamic)
      (Rendering|Material|SetScalarParameterValue Water%20Material "Breeze Offset" (Variables|ShoreParameters|GetBreeze%20Offset) :!class /Script/Engine.MaterialInstanceDynamic)
      (Rendering|Material|SetScalarParameterValue Water%20Material "Breeze Panning Speed" (Variables|ShoreParameters|GetBreeze%20Panning%20Speed) :!class /Script/Engine.MaterialInstanceDynamic)
      (Rendering|Material|SetScalarParameterValue Water%20Material "Breeze Power" (Variables|ShoreParameters|GetBreeze%20Power) :!class /Script/Engine.MaterialInstanceDynamic)
      (Rendering|Material|SetScalarParameterValue Water%20Material "Breeze Scale Distort" (Variables|ShoreParameters|GetBreeze%20Scale%20Distort) :!class /Script/Engine.MaterialInstanceDynamic))))