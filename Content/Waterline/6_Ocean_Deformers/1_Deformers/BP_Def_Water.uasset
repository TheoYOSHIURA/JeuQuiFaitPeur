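; Waterline ocean deformer volume that suppresses underwater post-processing and alters buoyancy and boat collision for whatever is inside its outer shell.
; Construction builds both shells and a flat skirt, copying tags and sim framerate from the ocean actor.
; Begin-play checks and overlap events toggle those effects.
; Player entry starts a timer micro-jittering the shells; JitterStop targets "Jitter Stop", so that timer keeps running.
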(event OnComponentBeginOverlap(Shell_Outer)
  (params (OverlappedComponent :type Primitive%20Component%20Object%20Reference) (OtherActor :type Actor%20Object%20Reference) (OtherComp :type Primitive%20Component%20Object%20Reference) (OtherBodyIndex :type Integer) (bFromSweep :type Boolean) (SweepResult :type Hit%20Result%20Structure%20%28by%20ref%29))
  (if (== OtherActor (Game|Player|GetPlayerPawn 0))
    (bind _returnvalue (Actor|GetActorOfClass "/Game/Waterline/3_Ocean_Sim_Content/BP_Waterline_Ocean_Gen_3.BP_Waterline_Ocean_Gen_3_C"))
    (Variables|/Script/Engine.PostProcessComponent|SetbEnabled (Variables|/Game/Waterline/3_Ocean_Sim_Content/BP_Waterline_Ocean_Gen_3.BP_Waterline_Ocean_Gen_3_C|GetUnderwater%20Post-Process%20Volume _returnvalue) false)
    (CallFunction|Jitter)
    (for _array_element (Class|PrimitiveComponent|GetOverlappingComponents (Variables|Default|GetShell_Outer))
      (if (or (Components|ComponentHasTag _array_element (Variables|Default|GetBuoyancy%20Advanced%20Tag)) (Components|ComponentHasTag _array_element (Variables|Default|GetBoat%20Tag)))
        (if (Actor|ActorHasTag (Components|GetOwner _array_element) "Boat")
          (Collision|SetCollisionEnabled _array_element "QueryOnly")
          (else
            (Collision|SetCollisionResponsetoChannel _array_element "ECC_GameTraceChannel1" "ECR_Ignore")))))
    (elif (or (Components|ComponentHasTag OtherComp (Variables|Default|GetBuoyancy%20Advanced%20Tag)) (Components|ComponentHasTag OtherComp (Variables|Default|GetBoat%20Tag)))
      (if (Actor|ActorHasTag OtherActor "Boat")
        (Collision|SetCollisionEnabled OtherComp "QueryOnly")
        (else
          (Collision|SetCollisionResponsetoChannel OtherComp "ECC_GameTraceChannel1" "ECR_Ignore"))))))

(event OnComponentEndOverlap(Shell_Outer)
  (params (OverlappedComponent :type Primitive%20Component%20Object%20Reference) (OtherActor :type Actor%20Object%20Reference) (OtherComp :type Primitive%20Component%20Object%20Reference) (OtherBodyIndex :type Integer))
  (if (== OtherActor (Game|Player|GetPlayerPawn 0))
    (bind _returnvalue (Actor|GetActorOfClass "/Game/Waterline/3_Ocean_Sim_Content/BP_Waterline_Ocean_Gen_3.BP_Waterline_Ocean_Gen_3_C"))
    (Variables|/Script/Engine.PostProcessComponent|SetbEnabled (Variables|/Game/Waterline/3_Ocean_Sim_Content/BP_Waterline_Ocean_Gen_3.BP_Waterline_Ocean_Gen_3_C|GetUnderwater%20Post-Process%20Volume _returnvalue) true)
    (CallFunction|JitterStop)
    (elif (or (Components|ComponentHasTag OtherComp (Variables|Default|GetBuoyancy%20Advanced%20Tag)) (Components|ComponentHasTag OtherComp (Variables|Default|GetBoat%20Tag)))
      (if (Actor|ActorHasTag OtherActor "Boat")
        (Collision|SetCollisionEnabled OtherComp "QueryAndPhysics")
        (else
          (Collision|SetCollisionResponsetoChannel OtherComp "ECC_GameTraceChannel1" "ECR_Overlap"))))))

(event Custom|Jitter
  (bind _shell_outer (Variables|Default|GetShell_Outer))
  (Utilities|Time|SetTimerbyFunctionName 0 "Jitter" (/ 1.0 (Variables|Default|GetOcean%20Sim%20Framerate)) true)
  (Utilities|FlowControl|FlipFlop
    (:A
      (Transformation|AddLocalOffset _shell_outer "0.000000,0.000000,0.000100" false false))
    (:B
      (Transformation|AddLocalOffset _shell_outer "0.000000,0.000000,-0.000100" false false))))

(event Custom|Jitter%20Stop
  (Class|KismetSystemLibrary|PauseTimer 0 "Jitter Stop"))

(event EventBeginPlay
  (bind _shell_outer (Variables|Default|GetShell_Outer))
  (bind _overlappingactors (Collision|GetOverlappingActors _shell_outer 0 :!class /Script/Engine.PrimitiveComponent))
  (Utilities|FlowControl|Delay 0.001)
  (if (> (Utilities|Array|Length _overlappingactors) 0)
    (if (Utilities|Array|ContainsItem _overlappingactors (Game|Player|GetPlayerPawn 0))
      (bind _returnvalue (Actor|GetActorOfClass "/Game/Waterline/3_Ocean_Sim_Content/BP_Waterline_Ocean_Gen_3.BP_Waterline_Ocean_Gen_3_C"))
      (Variables|/Script/Engine.PostProcessComponent|SetbEnabled (Variables|/Game/Waterline/3_Ocean_Sim_Content/BP_Waterline_Ocean_Gen_3.BP_Waterline_Ocean_Gen_3_C|GetUnderwater%20Post-Process%20Volume _returnvalue) false)
      (CallFunction|Jitter))
    (for _array_element (Class|PrimitiveComponent|GetOverlappingComponents (Variables|Default|GetShell_Outer))
      (if (or (Components|ComponentHasTag _array_element (Variables|Default|GetBuoyancy%20Advanced%20Tag)) (Components|ComponentHasTag _array_element (Variables|Default|GetBoat%20Tag)))
        (if (Actor|ActorHasTag (Components|GetOwner _array_element) "Boat")
          (Collision|SetCollisionEnabled _array_element "QueryOnly")
          (else
            (Collision|SetCollisionResponsetoChannel _array_element "ECC_GameTraceChannel1" "ECR_Ignore")))))))

(fn ConstructionScript
  (bind _deformer_skirt_scale (Variables|Default|GetDeformer%20Skirt%20Scale))
  (bind _shell_thickness (Variables|Default|GetShell%20Thickness))
  (bind _deformer_shape (Variables|Default|GetDeformer%20Shape))
  (bind _defaultsceneroot (Variables|Default|GetDefaultSceneRoot))
  (bind _returnvalue (Transformation|GetWorldScale _defaultsceneroot))
  (bind _returnvalue_2 (+ _returnvalue _deformer_skirt_scale))
  (bind _returnvalue_3 (Math|Float|Max(Float) (.x _returnvalue_2) (.y _returnvalue_2)))
  (Utilities|FlowControl|Sequence
    (:then_0
      (Components|StaticMesh|SetStaticMesh (Variables|Default|GetShell_Outer) _deformer_shape)
      (Components|StaticMesh|SetStaticMesh (Variables|Default|GetShell_Inner) _deformer_shape)
      (Rendering|Material|SetMaterial (Variables|Default|GetShell_Outer) 0 (Variables|Default|GetMaterial%20Outer))
      (Rendering|Material|SetMaterial (Variables|Default|GetShell_Inner) 0 (Variables|Default|GetMaterial%20Inner))
      (Rendering|Material|SetMaterial (Variables|Default|GetDF_Skirt) 0 "/Game/Waterline/6_Ocean_Deformers/2_Materials/M_Def_Skirt.M_Def_Skirt")
      (Transformation|SetWorldScale3D (Variables|Default|GetDF_Skirt) (Math|Vector|MakeVector _returnvalue_3 _returnvalue_3 0.0))
      (Transformation|SetWorldRotation (Variables|Default|GetDF_Skirt) "0, 0, 0" false false)
      (Transformation|SetRelativeScale3D (Variables|Default|GetShell_Outer) (Math|Vector|MakeVector _shell_thickness _shell_thickness _shell_thickness)))
    (:then_1
      (bind _returnvalue_4 (Actor|GetActorOfClass "/Game/Waterline/3_Ocean_Sim_Content/BP_Waterline_Ocean_Gen_3.BP_Waterline_Ocean_Gen_3_C"))
      (Variables|Default|SetBuoyancy%20Advanced%20Tag (Variables|/Game/Waterline/3_Ocean_Sim_Content/BP_Waterline_Ocean_Gen_3.BP_Waterline_Ocean_Gen_3_C|GetBuoyancy%20Advanced%20Tag _returnvalue_4))
      (Variables|Default|SetOcean%20Sim%20Framerate (Variables|/Game/Waterline/3_Ocean_Sim_Content/BP_Waterline_Ocean_Gen_3.BP_Waterline_Ocean_Gen_3_C|GetOcean%20Sim%20Framerate _returnvalue_4))
      (Variables|Default|SetBoat%20Tag (Variables|/Game/Waterline/3_Ocean_Sim_Content/BP_Waterline_Ocean_Gen_3.BP_Waterline_Ocean_Gen_3_C|GetBoat%20Tag _returnvalue_4)))))