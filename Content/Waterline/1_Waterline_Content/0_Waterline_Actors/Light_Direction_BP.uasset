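; Light direction actor for the Waterline content that writes the forward vector of Light1 into the Light_Direction material parameter collection as DIRACTION_1.
; The construction script and BeginPlay both write the value.
; UpdateLightDirection, started on BeginPlay, re-arms a looping timer on itself at the FPSUpdate rate and rewrites the vector on each call while DynamicUpdate is enabled.
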(event Custom|Update%20Light%20Direction
  (Utilities|Time|SetTimerbyEvent (delegate Custom|Update%20Light%20Direction) (/ 1.0 (Variables|Default|GetFPS%20Update)) true)
  (if (Variables|Default|GetDynamic%20Update)
    (Rendering|Material|SetVectorParameterValue "/Game/Waterline/1_Waterline_Content/Resources/Blueprints/Functions/Light_Direction.Light_Direction" "DIRACTION_1" (Math|Conversions|ToLinearColor(Vector) (Math|Vector|GetForwardVector (Variables|Default|GetLight_1))) :!class /Script/Engine.KismetMaterialLibrary)))

(event EventBeginPlay
  (CallFunction|UpdateLightDirection)
  (Rendering|Material|SetVectorParameterValue "/Game/Waterline/1_Waterline_Content/Resources/Blueprints/Functions/Light_Direction.Light_Direction" "DIRACTION_1" (Math|Conversions|ToLinearColor(Vector) (Math|Vector|GetForwardVector (Variables|Default|GetLight_1))) :!class /Script/Engine.KismetMaterialLibrary))

(fn ConstructionScript
  (Rendering|Material|SetVectorParameterValue "/Game/Waterline/1_Waterline_Content/Resources/Blueprints/Functions/Light_Direction.Light_Direction" "DIRACTION_1" (Math|Conversions|ToLinearColor(Vector) (Math|Vector|GetForwardVector (Variables|Default|GetLight_1))) :!class /Script/Engine.KismetMaterialLibrary))