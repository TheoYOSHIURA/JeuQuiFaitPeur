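; Free-flying camera pawn for moving freely through the scene.
; Movement axes add input along the control rotation's forward, right and up vectors, scaled by MovementSpeed.
; Each Tick consumes that input and applies it as an unswept world offset, so movement ignores collision and is not scaled by delta time.
; Mouse axes drive controller yaw and pitch.
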(event EventTick
  (params (DeltaSeconds :type Float%20%28single-precision%29))
  ;[1 1 1] Camera Control
  (bind _returnvalue (Class|Pawn|ConsumeMovementInputVector))
  (Transformation|AddActorWorldOffset _returnvalue))

(event Input|AxisEvents|InputAxisMoveForward
  (params (AxisValue :type Float%20%28single-precision%29))
  ;[1 1 1] Camera Control
  ;;[1 1 1] Keyboard
  (Pawn|Input|AddMovementInput (Math|Vector|GetForwardVector (Pawn|GetControlRotation :!class /Script/Engine.Pawn)) (* AxisValue (Variables|Default|GetMovement%20Speed)) false))

(event Input|AxisEvents|InputAxisMoveRight
  (params (AxisValue :type Float%20%28single-precision%29))
  ;[1 1 1] Camera Control
  ;;[1 1 1] Keyboard
  (Pawn|Input|AddMovementInput (Math|Vector|GetRightVector (Pawn|GetControlRotation :!class /Script/Engine.Pawn)) (* AxisValue (Variables|Default|GetMovement%20Speed)) false))

(event Input|AxisEvents|InputAxisMoveUp
  (params (AxisValue :type Float%20%28single-precision%29))
  ;[1 1 1] Camera Control
  ;;[1 1 1] Keyboard
  (Pawn|Input|AddMovementInput (Math|Vector|GetUpVector (Pawn|GetControlRotation :!class /Script/Engine.Pawn)) (* AxisValue (Variables|Default|GetMovement%20Speed)) false))

(event Input|AxisEvents|InputAxisRotationX
  (params (AxisValue :type Float%20%28single-precision%29))
  ;[1 1 1] Camera Control
  ;;[1 1 1] Mouse
  (Pawn|Input|AddControllerYawInput AxisValue))

(event Input|AxisEvents|InputAxisRotationY
  (params (AxisValue :type Float%20%28single-precision%29))
  ;[1 1 1] Camera Control
  ;;[1 1 1] Mouse
  (Pawn|Input|AddControllerPitchInput AxisValue))

(fn ConstructionScript)